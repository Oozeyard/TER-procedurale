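; Blueprint that randomizes the generator parameters of a referenced Planet every frame, apparently to vary its procedural shape.
; On each Tick it writes new random values for frequency, noise seed and noise strength into the Planet's Generator picker by parameter name.
; It only sets parameters, with no explicit rebuild call, and its construction script is empty.
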(event `self.ReceiveTick`
  (params (DeltaSeconds :type "Float (single-precision)"))
  (`VoxelGeneratorTools.SetGeneratorParameter` (`VoxelWorld.Generator` (`self.Planet`)) "Frequency" (`KismetMathLibrary.RandomFloat`))
  (`VoxelGeneratorTools.SetGeneratorParameter` (`VoxelWorld.Generator` (`self.Planet`)) "Noise_Seed" (`KismetMathLibrary.RandomInteger` 5000))
  (`VoxelGeneratorTools.SetGeneratorParameter` (`VoxelWorld.Generator` (`self.Planet`)) "Noise_Strength" (`KismetMathLibrary.RandomFloat`)))

(fn `UserConstructionScript`)