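; BP_ExemplePlanet is an example procedural planet that builds a randomized voxel world when play begins.
; On BeginPlay it casts the Planet child actor to VoxelWorld and randomizes the generator's frequency, noise seed and noise strength parameters.
; It then calls CreateWorld, so the terrain is generated at runtime from those random values, with zero frequency noted as a flat surface.
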(event `self.ReceiveBeginPlay`
  (bind _asvoxel_world (cast `VoxelWorld` (`ChildActorComponent.ChildActor` (`self.Planet`))))
  ;[1 1 1] Frequency : 0 == flat surface
  (`VoxelGeneratorTools.SetGeneratorParameter` (`VoxelWorld.Generator` _asvoxel_world) "Frequency" (`KismetMathLibrary.RandomFloat`))
  ;[1 1 1] Seed
  (`VoxelGeneratorTools.SetGeneratorParameter` (`VoxelWorld.Generator` _asvoxel_world) "Noise_Seed" (`KismetMathLibrary.RandomInteger` 5000))
  (`VoxelGeneratorTools.SetGeneratorParameter` (`VoxelWorld.Generator` _asvoxel_world) "Noise_Strength" (`KismetMathLibrary.RandomFloat`))
  (`VoxelWorld.CreateWorld` :`self` _asvoxel_world))

(fn `UserConstructionScript`)