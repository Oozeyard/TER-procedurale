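; BP_Terrain is a procedural terrain actor that builds a grid mesh with collision and a material in its construction script.
; GenerateSurface fills vertices, UVs and triangle indices, calculates normals and tangents, then creates the mesh section.
; GetHeight multiplies two scaled 1D Perlin noise samples, one per axis, with no random seed.
; Pressing R at runtime clears the arrays and rebuilds the surface.
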(event `self.ReceiveBeginPlay`
  (`self.EnableInput` (`GameplayStatics.GetPlayerController` 0)))

(event `Key|R`
  (params (Key :type "Key Structure"))
  (:`Pressed`
    (`KismetSystemLibrary.PrintText` "Regenerate")
    (`KismetArrayLibrary.Array_Clear` (`self.Vertices`))
    (`KismetArrayLibrary.Array_Clear` (`self.Triangles`))
    (`KismetArrayLibrary.Array_Clear` (`self.UV0`))
    (`self.Generate Surface`)))

(fn `Generate Surface`
  (bind _xsize (`self.XSize`))
  (bind _cellsize (`self.CellSize`))
  (bind _triangles (`self.Triangles`))
  (bind _triangles_2 (`self.Triangles`))
  ;[1 1 1] Generate vertices
  (for _index (range (`self.XSize`))
    (for _index_2 (range (`self.YSize`))
      (bind _returnvalue (* _index_2 _cellsize))
      (bind _returnvalue_2 (* _index _cellsize))
      (`KismetArrayLibrary.Array_Add` (`self.Vertices`) (`KismetMathLibrary.MakeVector` _returnvalue _returnvalue_2 (`self.GetHeight` _returnvalue _returnvalue_2)))
      ;[1 1 1] UVs
      (`KismetArrayLibrary.Array_Add` (`self.UV0`) (`KismetMathLibrary.MakeVector2D` (`KismetMathLibrary.Conv_IntToDouble` _index) (`KismetMathLibrary.Conv_IntToDouble` _index_2)))))
  ;[1 1 1] Generate triangles
  (for _index_3 (range 1 (+ (- (`self.XSize`) 2) 1))
    (for _index_4 (range 1 (+ (- (`self.YSize`) 2) 1))
      (bind _returnvalue_3 (+ _index_3 (* _index_4 _xsize)))
      (`KismetArrayLibrary.Array_Add` _triangles _returnvalue_3)
      (bind _returnvalue_4 (+ _returnvalue_3 _xsize))
      (`KismetArrayLibrary.Array_Add` _triangles _returnvalue_4)
      (bind _returnvalue_5 (+ _returnvalue_3 1))
      (`KismetArrayLibrary.Array_Add` _triangles _returnvalue_5)
      (`KismetArrayLibrary.Array_Add` _triangles_2 _returnvalue_4)
      (`KismetArrayLibrary.Array_Add` _triangles_2 (+ _returnvalue_4 1))
      (`KismetArrayLibrary.Array_Add` _triangles_2 _returnvalue_5)))
  (bind (_normals _tangents) (`KismetProceduralMeshLibrary.CalculateTangentsForMesh` (`self.Vertices`) (`self.Triangles`) (`self.UV0`)))
  (`ProceduralMeshComponent.CreateMeshSection_LinearColor` :`self` (`self.TerrainMesh`) :`Vertices` (`self.Vertices`) :`Triangles` (`self.Triangles`) :`Normals` _normals :`UV0` (`self.UV0`) :`Tangents` _tangents :`bCreateCollision` true)
  (`PrimitiveComponent.SetMaterial` (`self.TerrainMesh`) 0 (`self.Material`)))

(fn `GetHeight`
  (params (X :type "Float (double-precision)") (Y :type "Float (double-precision)"))
  (returns (Z :type "Float (double-precision)"))
  (return (* (* (`KismetMathLibrary.PerlinNoise1D` (+ X 0.1)) (`KismetMathLibrary.PerlinNoise1D` (+ Y 0.1))) 2000.0)))

(fn `UserConstructionScript`
  (`self.Generate Surface`))