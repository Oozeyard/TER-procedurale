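; Earth map camera that becomes the player's view on BeginPlay and turns left clicks on the map into level loads.
; A click line-traces from the cursor, draws the hit component's material to a temporary render target and reads the color at the hit UV.
; That color is matched exactly against MapArray's values, and the corresponding key names the level to open, making the material a color-coded picking mask.
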(event `self.ReceiveBeginPlay`
  (bind _returnvalue (`GameplayStatics.GetPlayerController` 0))
  (`self.EnableInput` _returnvalue)
  (`PlayerController.SetViewTargetWithBlend` _returnvalue self 0.0 "VTBlend_Linear" 0.0 false))

(event `Key|LeftMouseButton`
  (params (Key :type "Key Structure"))
  (bind _maparray (`self.MapArray`))
  (bind (_worldlocation _worlddirection) (`PlayerController.DeprojectMousePositionToWorld` (`GameplayStatics.GetPlayerController` 0)))
  ;[1 1 1] Get Hit point
  (:`Pressed`
    (bind _outhit (`KismetSystemLibrary.LineTraceSingle` _worldlocation (+ _worldlocation (* _worlddirection 7000.0)) "TraceTypeQuery1" true))
    ;[1 1 1] Get Material
    (bind _returnvalue (`KismetRenderingLibrary.CreateRenderTarget2D` 255 255 "RTF_RGBA8" (struct :`A` 1.0) false true))
    (`KismetRenderingLibrary.DrawMaterialToRenderTarget` _returnvalue (`PrimitiveComponent.GetMaterial` (`.HitComponent` (`GameplayStatics.BreakHitResult` _outhit)) 0))
    (bind (_x _y) (`KismetMathLibrary.BreakVector2D` (`GameplayStatics.FindCollisionUV` _outhit)))
    ;[1 1 1] Return color based on UV
    (bind _returnvalue_2 (`KismetRenderingLibrary.ReadRenderTargetRawUV` _returnvalue _x _y))
    (bind _values (`BlueprintMapLibrary.Map_Values` _maparray))
    (bind _keys (`BlueprintMapLibrary.Map_Keys` _maparray))
    (bind (_r _g _b) (`KismetMathLibrary.BreakColor` _returnvalue_2))
    (`GameplayStatics.OpenLevel` (`KismetStringLibrary.Conv_StringToName` (`|GetArrayItem` _keys (`KismetArrayLibrary.Array_Find` _values (`KismetMathLibrary.MakeVector` _r _g _b)))))))

(fn `UserConstructionScript`)