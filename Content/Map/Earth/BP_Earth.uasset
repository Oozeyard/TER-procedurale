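; Earth map-selection actor that takes over the player's view and opens a level when the clicked surface colour matches a map entry.
; Held keys pan, zoom and roll its camera through self-repeating short-delay loops.
; A left click line-traces under the cursor, draws the hit material to a render target and reads the colour at the hit UV.
; That colour is looked up in MapArray to find the level name.
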(event `self.ReceiveBeginPlay`
  (bind _returnvalue (`GameplayStatics.GetPlayerController` 0))
  (`self.EnableInput` _returnvalue)
  (`PlayerController.SetViewTargetWithBlend` _returnvalue self 0.0 "VTBlend_Linear" 0.0 false))

(event `TranslationLeft`
  ;[1 1 1] Translation
  (`SceneComponent.K2_AddRelativeLocation` (`self.Camera`) (0.0 -10.0 0.0) false false :!label _label)
  (if (`self.translateRightLeft`)
    (`KismetSystemLibrary.Delay` 0.01)
    (goto _label)))

(event `TranslationRight`
  ;[1 1 1] Translation
  (`SceneComponent.K2_AddRelativeLocation` (`self.Camera`) (0.0 10.0 0.0) false false :!label _label_2)
  (if (`self.translateRightLeft`)
    (`KismetSystemLibrary.Delay` 0.01)
    (goto _label_2)))

(event `ZoomIn`
  ;[1 1 1] Translation
  (`SceneComponent.K2_AddRelativeLocation` (`self.Camera`) (5.0 0.0 0.0) false false :!label _label_3)
  (if (`self.translateInOut`)
    (`KismetSystemLibrary.Delay` 0.01)
    (goto _label_3)))

(event `ZoomOut`
  ;[1 1 1] Translation
  (`SceneComponent.K2_AddRelativeLocation` (`self.Camera`) (-5.0 0.0 0.0) false false :!label _label_4)
  (if (`self.translateInOut`)
    (`KismetSystemLibrary.Delay` 0.01)
    (goto _label_4)))

(event `RotateLeft`
  ;[1 1 1] Rotate camera
  (`SceneComponent.K2_AddLocalRotation` (`self.Camera`) (struct :`Yaw` 0.5) false false :!label _label_5)
  (if (`self.rotate`)
    (`KismetSystemLibrary.Delay` 0.01)
    (goto _label_5)))

(event `Key|Q`
  (params (Key :type "Key Structure"))
  ;[1 1 1] Translation
  (:`Pressed`
    (set `self.translateRightLeft` true)
    (`self.TranslationLeft`))
  (:`Released`
    (set `self.translateRightLeft` false :!label _label_6)))

(event `Key|D`
  (params (Key :type "Key Structure"))
  ;[1 1 1] Translation
  (:`Pressed`
    (set `self.translateRightLeft` true)
    (`self.TranslationRight`))
  (:`Released`
    (goto _label_6)))

(event `RotateRight`
  ;[1 1 1] Rotate camera
  (`SceneComponent.K2_AddLocalRotation` (`self.Camera`) (struct :`Yaw` -0.5) false false :!label _label_7)
  (if (`self.rotate`)
    (`KismetSystemLibrary.Delay` 0.01)
    (goto _label_7)))

(event `Key|E`
  (params (Key :type "Key Structure"))
  ;[1 1 1] Rotate camera
  (:`Pressed`
    (set `self.rotate` true)
    (`self.RotateLeft`))
  (:`Released`
    (set `self.rotate` false :!label _label_8)))

(event `Key|Z`
  (params (Key :type "Key Structure"))
  ;[1 1 1] Translation
  (:`Pressed`
    (set `self.translateInOut` true)
    (`self.ZoomIn`))
  (:`Released`
    (set `self.translateInOut` false :!label _label_9)))

(event `Key|A`
  (params (Key :type "Key Structure"))
  ;[1 1 1] Rotate camera
  (:`Pressed`
    (set `self.rotate` true)
    (`self.RotateRight`))
  (:`Released`
    (goto _label_8)))

(event `Key|S`
  (params (Key :type "Key Structure"))
  ;[1 1 1] Translation
  (:`Pressed`
    (set `self.translateInOut` true)
    (`self.ZoomOut`))
  (:`Released`
    (goto _label_9)))

(event `Key|LeftMouseButton`
  (params (Key :type "Key Structure"))
  (bind _maparray (`self.MapArray`))
  (bind (_worldlocation _worlddirection) (`PlayerController.DeprojectMousePositionToWorld` (`GameplayStatics.GetPlayerController` 0)))
  ;[1 1 1] Get Hit point
  (:`Pressed`
    (bind _outhit (`KismetSystemLibrary.LineTraceSingle` _worldlocation (+ _worldlocation (* _worlddirection 7000.0)) "TraceTypeQuery1" true))
    (bind (_bblockinghit _binitialoverlap _time _distance _location _impactpoint _normal _impactnormal _physmat _hitactor _hitcomponent) (`GameplayStatics.BreakHitResult` _outhit))
    ;[1 1 1] Get Material
    (`/Engine/EditorBlueprintResources/StandardMacros.IsValid` _hitcomponent
      (:`Is Valid`
        (bind _returnvalue (`KismetRenderingLibrary.CreateRenderTarget2D` 255 255 "RTF_RGBA8" (struct :`A` 1.0) false true))
        (`KismetRenderingLibrary.DrawMaterialToRenderTarget` _returnvalue (`PrimitiveComponent.GetMaterial` _hitcomponent 0))
        (bind (_x _y) (`KismetMathLibrary.BreakVector2D` (`GameplayStatics.FindCollisionUV` _outhit)))
        ;[1 1 1] Return color based on UV
        (bind _returnvalue_2 (`KismetRenderingLibrary.ReadRenderTargetRawUV` _returnvalue _x _y))
        ;[1 1 1] Open map based on color
        (bind _values (`BlueprintMapLibrary.Map_Values` _maparray))
        (bind _keys (`BlueprintMapLibrary.Map_Keys` _maparray))
        (bind (_r _g _b) (`KismetMathLibrary.BreakColor` _returnvalue_2))
        (bind _returnvalue_3 (`KismetArrayLibrary.Array_Find` _values (`KismetMathLibrary.MakeVector` _r _g _b)))
        ;;[1 1 1] not a map
        (if (!= -1 _returnvalue_3)
          (`GameplayStatics.OpenLevel` (`KismetStringLibrary.Conv_StringToName` (`|GetArrayItem` _keys _returnvalue_3))))))))

(fn `UserConstructionScript`)