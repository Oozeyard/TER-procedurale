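; BP_Sphere is an Earth globe actor that the player rotates by click-dragging.
; It enables input from player controller 0 on BeginPlay, and click and release events on the Earth component toggle a dragging flag.
; While dragging, mouse X and Y axis input add inverted, scaled yaw and pitch to the actor's rotation through CombineRotators.
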(event `self.ReceiveBeginPlay`
  (`self.EnableInput` (`GameplayStatics.GetPlayerController` 0)))

(event `self.ReceiveTick`
  (params (DeltaSeconds :type "Float (single-precision)")))

(event `self.Earth.OnReleased`
  (params (TouchedComponent :type "PrimitiveComponent Object Reference") (ButtonReleased :type "Key Structure"))
  (set `self.isDragging` false))

(event `self.Earth.OnClicked`
  (params (TouchedComponent :type "PrimitiveComponent Object Reference") (ButtonPressed :type "Key Structure"))
  (set `self.isDragging` true))

(event `InputAxisKey|MouseX`
  (params (AxisValue :type "Float (single-precision)"))
  (if (`self.isDragging`)
    (`self.K2_SetActorRotation` (`KismetMathLibrary.ComposeRotators` (`self.K2_GetActorRotation`) (`KismetMathLibrary.MakeRotator` 0.0 0.0 (* AxisValue -3.0))))))

(event `InputAxisKey|MouseY`
  (params (AxisValue :type "Float (single-precision)"))
  (if (`self.isDragging`)
    (`self.K2_SetActorRotation` (`KismetMathLibrary.ComposeRotators` (`self.K2_GetActorRotation`) (`KismetMathLibrary.MakeRotator` 0.0 (* AxisValue -3.0))))))

(fn `UserConstructionScript`)